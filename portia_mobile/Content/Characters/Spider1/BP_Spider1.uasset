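; Spider character Blueprint that grows gradually from a baby by scaling itself up over time.
; On BeginPlay it starts a looping GrowUpBaby timer with a random interval of a few seconds, chosen once per spider.
; Each call raises GrowSize by a small step until just past full size, applying it as uniform scale and printing debug output.
; BeginPlay also caches all BP_Spider1_Object actors as ExitPoints, unused here.
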(event `GrowingUpBaby`)

(event `self.ReceiveBeginPlay`
  (`KismetSystemLibrary.K2_SetTimer` null "GrowUpBaby" (`KismetMathLibrary.RandomFloatInRange` 3.0 5.0) true)
  (bind _outactors (`GameplayStatics.GetAllActorsOfClass` "/Game/Characters/Spider1/BP_Spider1_Object.BP_Spider1_Object_C"))
  (set `self.ExitPoints` _outactors))

(fn `GrowUpBaby`
  (bind _growsize (`self.GrowSize`))
  (if (<= (`self.GrowSize`) 1.0)
    (`KismetSystemLibrary.PrintString` (`KismetStringLibrary.Conv_DoubleToString` _growsize))
    (set `self.GrowSize` (+ _growsize 0.025))
    (`self.SetActorScale3D` (+ (`KismetMathLibrary.MakeVector` _growsize _growsize _growsize) (0.025 0.025 0.025)))))

(fn `UserConstructionScript`)